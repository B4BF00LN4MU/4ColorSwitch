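; BP_SwitchTrigger is an escape-room trigger that presents a switch puzzle and opens a linked door when it is answered correctly.
; Overlapping its Box creates a BP_Switch_UI widget, shows the cursor, switches to UI-only input and pauses the game.
; The widget's right-answer callback closes it, restores game input, unpauses, opens DoorActor and destroys the Box.
; Ending the overlap removes the widget, hides the cursor and unpauses.
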(event OnComponentBeginOverlap(Box)
  (params (OverlappedComponent :type Primitive%20Component%20Object%20Reference) (OtherActor :type Actor%20Object%20Reference) (OtherComp :type Primitive%20Component%20Object%20Reference) (OtherBodyIndex :type Integer) (bFromSweep :type Boolean) (SweepResult :type Hit%20Result%20Structure%20%28by%20ref%29))
  (bind _returnvalue (Game|GetPlayerController 0))
  (bind _returnvalue_2 (UserInterface|CreateWidget "/EscapeTool/EscapeRoom/Widget/BP_Switch_UI.BP_Switch_UI_C"))
  (Variables|Default|SetSwitchUI _returnvalue_2)
  (EventDispatchers|BindEventtoOnAnswerIsRight (Variables|Default|GetSwitchUI) (EventDispatchers|CreateEvent :!event OnAnswerIsRight))
  (Variables|/Script/Engine.PlayerController|SetbShowMouseCursor _returnvalue true)
  (Input|SetInputModeUIOnly _returnvalue 0 "DoNotLock" false)
  (UserInterface|Viewport|AddtoViewport (Variables|Default|GetSwitchUI) 0)
  (Game|SetGamePaused true))

(event OnComponentEndOverlap(Box)
  (params (OverlappedComponent :type Primitive%20Component%20Object%20Reference) (OtherActor :type Actor%20Object%20Reference) (OtherComp :type Primitive%20Component%20Object%20Reference) (OtherBodyIndex :type Integer))
  (Variables|/Script/Engine.PlayerController|SetbShowMouseCursor (Game|GetPlayerController 0) false)
  (Widget|RemovefromParent (Variables|Default|GetSwitchUI))
  (Game|SetGamePaused false))

(fn ConstructionScript)

(fn OnAnswerIsRight
  (params (NewParam :type Integer))
  (bind _returnvalue (Game|GetPlayerController 0))
  (Widget|RemovefromParent (Variables|Default|GetSwitchUI))
  (Variables|/Script/Engine.PlayerController|SetbShowMouseCursor _returnvalue false)
  (Input|SetInputModeGameOnly _returnvalue false)
  (Game|SetGamePaused false)
  (Default|DoOpenDoor (Variables|Default|GetDoorActor))
  (Components|DestroyComponent (Variables|Default|GetBox)))